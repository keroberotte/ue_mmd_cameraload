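; BP_CameraMover drives a camera in sync with an MMD model's animation, following MMD-style pivot, rotation, distance and field-of-view data.
; Each tick it converts the skeletal mesh's playback position to a frame number at 30 fps and samples the camera values for that frame.
; The actor takes the pivot's location and rotation, while the child CameraActor takes the field of view and local X distance, with distances scaled by 8.
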(event `self.ReceiveTick`
  (params (DeltaSeconds :type "Float (single-precision)"))
  (bind _returnvalue (* (`SkeletalMeshComponent.GetPosition` (`SkeletalMeshActor.SkeletalMeshComponent` (`self.MMDModel`))) 30.0))
  ;[1 1 1] Get Frame Position
  ;[0.1095 1 0] Set parent pos and rot
  (bind _returnvalue_2 (`self.getPos` _returnvalue))
  (bind _returnvalue_3 (`self.getRot` _returnvalue))
  (`self.K2_SetActorLocationAndRotation` (* _returnvalue_2 8.0) _returnvalue_3)
  ;[0.1095 1 0] Set child pos and rot
  (bind `_asカメラアクタ` (cast `CameraActor` (`ChildActorComponent.ChildActor` (`self.CameraActor`))))
  (bind _returnvalue_4 (`self.getFov` _returnvalue))
  (`CameraComponent.SetFieldOfView` (`CameraActor.CameraComponent` `_asカメラアクタ`) _returnvalue_4)
  (bind _returnvalue_5 (`self.getDistance` _returnvalue))
  (`SceneComponent.K2_SetRelativeLocation` (`self.CameraActor`) (`KismetMathLibrary.MakeVector` (* _returnvalue_5 8.0)) false false))

(fn `UserConstructionScript`)